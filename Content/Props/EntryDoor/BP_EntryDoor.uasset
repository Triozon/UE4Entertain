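; Entry door Blueprint: a locked double door that the player opens with a key and the action key, which then starts the ExplainObjectives level sequence.
; A box trigger checks the ThirdPersonCharacter for the key and shows a prompt or missing-key message on a text render.
; While the player stays in the box, a delay loop polls for the action key.
; Unlocking plays sounds, then rotates both door meshes open with MoveComponentTo.
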(event `self.Box.OnComponentBeginOverlap`
  (params (OverlappedComponent :type "PrimitiveComponent Object Reference") (OtherActor :type "Actor Object Reference") (OtherComp :type "PrimitiveComponent Object Reference") (OtherBodyIndex :type Integer) (bFromSweep :type Boolean) (SweepResult :type "HitResult Structure (by ref)"))
  (bind _sm_door_3_1 (`self.SM_Door_3_1`))
  (bind _sm_door_3_2 (`self.SM_Door_3_2`))
  (bind _returnvalue (`SceneComponent.K2_GetComponentLocation` (`self.SM_Door_3_1`)))
  (bind _relativelocation (`SceneComponent.RelativeLocation` _sm_door_3_1))
  (set `self.IsInFrontOfDoor` true)
  (if (not (`self.Open`))
    (`/Engine/EditorBlueprintResources/StandardMacros.DoOnce` false :!label _label
      (:`Completed`
        (bind _asthird_person_character (cast `/Game/ThirdPersonBP/Blueprints/ThirdPersonCharacter` OtherActor))
        (if (`/Game/ThirdPersonBP/Blueprints/ThirdPersonCharacter.HaveEntryDoorKey` _asthird_person_character)
          (if (`/Game/ThirdPersonBP/Blueprints/ThirdPersonCharacter.UseActionKey` _asthird_person_character) :!label _label_2
            (`GameplayStatics.PlaySoundAtLocation` "/Game/Props/EntryDoor/Unlocking_door.Unlocking_door" _returnvalue (struct) 1.0 1.0 0.0 null null null)
            (`KismetSystemLibrary.Delay` 6.0)
            (`GameplayStatics.PlaySoundAtLocation` "/Game/Props/grincement_porte_metal.grincement_porte_metal" _returnvalue (struct) 1.0 1.0 0.0 null null null)
            (`KismetSystemLibrary.MoveComponentTo` _sm_door_3_2 (`SceneComponent.RelativeLocation` _sm_door_3_2) (`KismetMathLibrary.MakeRotator` (.roll (`SceneComponent.RelativeRotation` _sm_door_3_2)) (.pitch (`SceneComponent.RelativeRotation` _sm_door_3_2)) 90.0) true false 1.0)
            (`GameplayStatics.PlaySoundAtLocation` "/Game/Props/grincement_porte_metal.grincement_porte_metal" _relativelocation (struct) 1.0 1.0 0.0 null null null)
            (`KismetSystemLibrary.MoveComponentTo` _sm_door_3_1 _relativelocation (`KismetMathLibrary.MakeRotator` (.roll (`SceneComponent.RelativeRotation` _sm_door_3_1)) (.pitch (`SceneComponent.RelativeRotation` _sm_door_3_1)) -90.0) true true 1.0 true)
            (`TextRenderComponent.K2_SetText` (`self.TextRender`) (`KismetTextLibrary.Conv_StringToText` ""))
            (`KismetSystemLibrary.Delay` 0.2)
            (set `self.Open` true)
            (bind _outactor (`LevelSequencePlayer.CreateLevelSequencePlayer` "/Game/Props/EntryDoor/ExplainObjectives.ExplainObjectives"))
            (`MovieSceneSequencePlayer.Play` (`LevelSequenceActor.SequencePlayer` _outactor))
            (elif (`self.IsInFrontOfDoor`)
              (`TextRenderComponent.K2_SetText` (`self.TextRender`) (`KismetTextLibrary.Conv_StringToText` "Press action Keyto use Keys \n(default on F) "))
              (`KismetSystemLibrary.Delay` 0.2)
              (goto _label_2)
              (else
                (goto _label :!via `Reset`))))
          (else
            (`TextRenderComponent.K2_SetText` (`self.TextRender`) (`KismetTextLibrary.Conv_StringToText` "You dont have the Key"))
            (goto _label :!via `Reset`)))))))

(event `self.Box.OnComponentEndOverlap`
  (params (OverlappedComponent :type "PrimitiveComponent Object Reference") (OtherActor :type "Actor Object Reference") (OtherComp :type "PrimitiveComponent Object Reference") (OtherBodyIndex :type Integer))
  (set `self.IsInFrontOfDoor` false)
  (`TextRenderComponent.K2_SetText` (`self.TextRender`) (`KismetTextLibrary.Conv_StringToText` ""))
  (`KismetSystemLibrary.Delay` 0.2)
  (goto _label :!via `Reset`))

(fn `UserConstructionScript`)