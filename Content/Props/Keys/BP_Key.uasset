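; BP_Key is a key pickup prop that grants the player the entry door key when a ThirdPersonCharacter overlaps its box.
; On overlap it sets the character's HaveEntryDoorKey flag, plays a pickup sound and destroys its box, key and root components.
; It then calls DisableInput with the player controller, plays a level sequence, and calls EnableInput after a fixed delay.
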(event `self.Box.OnComponentBeginOverlap`
  (params (OverlappedComponent :type "PrimitiveComponent Object Reference") (OtherActor :type "Actor Object Reference") (OtherComp :type "PrimitiveComponent Object Reference") (OtherBodyIndex :type Integer) (bFromSweep :type Boolean) (SweepResult :type "HitResult Structure (by ref)"))
  (bind _returnvalue (`GameplayStatics.GetPlayerController` 0))
  (bind _asthird_person_character (cast `/Game/ThirdPersonBP/Blueprints/ThirdPersonCharacter` OtherActor))
  (set `/Game/ThirdPersonBP/Blueprints/ThirdPersonCharacter.HaveEntryDoorKey` true _asthird_person_character)
  (`GameplayStatics.PlaySoundAtLocation` "/Game/Props/Keys/PickKeySound.PickKeySound" (`SceneComponent.K2_GetComponentLocation` (`self.DefaultSceneRoot`)) (struct) 1.0 1.0 0.0 null null null)
  (`ActorComponent.K2_DestroyComponent` (`self.Box`))
  (`ActorComponent.K2_DestroyComponent` (`self.Key`))
  (`ActorComponent.K2_DestroyComponent` (`self.DefaultSceneRoot`))
  (`self.DisableInput` _returnvalue)
  (bind _outactor (`LevelSequencePlayer.CreateLevelSequencePlayer` (`self.LevelSequence`)))
  (`MovieSceneSequencePlayer.Play` (`LevelSequenceActor.SequencePlayer` _outactor))
  (`KismetSystemLibrary.Delay` 5.0)
  (`self.EnableInput` _returnvalue))

(fn `UserConstructionScript`)