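; Keypad-operated door that swings open when a ThirdPersonCharacter inside its trigger has UseActionKey set, with a text display of the time left.
; While the character waits in DetectPlayer, a delay loop polls the key and blinks the keypad by swapping materials.
; Opening rotates the door 90 degrees and counts down Seconds, then closes it and resets the timer.
; An initial time of zero leaves the door open and shows the Infinite text.
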(event `self.ReceiveBeginPlay`
  (bind _timeleft (`self.TimeLeft`))
  (bind _output_get (set `self.InitSecond` (`self.Seconds`)))
  (if (> _output_get 0.0)
    (`TextRenderComponent.K2_SetText` _timeleft (`KismetTextLibrary.Conv_DoubleToText` _output_get "HalfToEven"))
    (else
      (`TextRenderComponent.K2_SetText` _timeleft (`self.Infinite`)))))

(event `self.DetectPlayer.OnComponentBeginOverlap`
  (params (OverlappedComponent :type "PrimitiveComponent Object Reference") (OtherActor :type "Actor Object Reference") (OtherComp :type "PrimitiveComponent Object Reference") (OtherBodyIndex :type Integer) (bFromSweep :type Boolean) (SweepResult :type "HitResult Structure (by ref)"))
  (bind _sm_door_1 (`self.SM_Door_1`))
  (bind _timeleft (`self.TimeLeft`))
  (bind _sm_door_1_2 (`self.SM_Door_1`))
  (bind _sm_door_1_3 (`self.SM_Door_1`))
  ;[1 1 1] keypad activation+ open door
  (bind _asthird_person_character (cast `/Game/ThirdPersonBP/Blueprints/ThirdPersonCharacter` OtherActor))
  (set `self.PlayerinFront?` true)
  (if (`self.PlayerinFront?`) :!label _label
    (bind _useactionkey (`/Game/ThirdPersonBP/Blueprints/ThirdPersonCharacter.UseActionKey` _asthird_person_character))
    (if _useactionkey
      (`PrimitiveComponent.CreateDynamicMaterialInstance` (`self.keypad`) 0 "/Game/IndustrialArea/Materials/M_Wall_Elements.M_Wall_Elements" "None")
      (`KismetSystemLibrary.MoveComponentTo` _sm_door_1_2 (`SceneComponent.RelativeLocation` _sm_door_1) (`KismetMathLibrary.MakeRotator` (.roll (`SceneComponent.RelativeRotation` _sm_door_1)) (.pitch (`SceneComponent.RelativeRotation` _sm_door_1)) 90.0) true true 1.0 true)
      (if (> (`self.Seconds`) 0.1) :!label _label_2
        (`KismetSystemLibrary.Delay` 1.0)
        (bind _output_get (set `self.Seconds` (- (`self.Seconds`) 1.0)))
        (`TextRenderComponent.K2_SetText` _timeleft (`KismetTextLibrary.Conv_DoubleToText` _output_get "HalfToEven"))
        (goto _label_2)
        (elif (== (`self.InitSecond`) 0.0)
          (goto _label)
          (else
            (`KismetSystemLibrary.MoveComponentTo` _sm_door_1_2 (`SceneComponent.RelativeLocation` _sm_door_1_3) (`KismetMathLibrary.MakeRotator` (.roll (`SceneComponent.RelativeRotation` _sm_door_1_3)) (.pitch (`SceneComponent.RelativeRotation` _sm_door_1_3))) true true 1.0 true)
            (`KismetSystemLibrary.Delay` 1.0)
            (bind _output_get_2 (set `self.Seconds` (`self.InitSecond`)))
            (`TextRenderComponent.K2_SetText` _timeleft (`KismetTextLibrary.Conv_DoubleToText` _output_get_2 "HalfToEven"))
            (goto _label))))
      (else
        (`PrimitiveComponent.CreateDynamicMaterialInstance` (`self.keypad`) 0 "/Game/StarterContent/Materials/M_Glass.M_Glass" "None")
        (`KismetSystemLibrary.Delay` 0.5)
        (if _useactionkey
          _
          (else
            _))
        (`PrimitiveComponent.CreateDynamicMaterialInstance` (`self.keypad`) 0 "/Game/IndustrialArea/Materials/M_Wall_Elements.M_Wall_Elements" "None")
        (`KismetSystemLibrary.Delay` 0.5)
        (goto _label)))))

(event `self.DetectPlayer.OnComponentEndOverlap`
  (params (OverlappedComponent :type "PrimitiveComponent Object Reference") (OtherActor :type "Actor Object Reference") (OtherComp :type "PrimitiveComponent Object Reference") (OtherBodyIndex :type Integer))
  ;[1 1 1] keypad activation+ open door
  (cast `/Game/ThirdPersonBP/Blueprints/ThirdPersonCharacter` OtherActor)
  (set `self.PlayerinFront?` false))

(fn `UserConstructionScript`)